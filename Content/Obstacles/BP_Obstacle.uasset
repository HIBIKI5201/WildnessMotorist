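; Obstacle actor that grades an overlapping actor by its lateral (local Y) distance from the obstacle's center.
; GetRegionValue returns the first score definition in Def whose distance covers that offset, falling back to the last; on overlap the result is only printed in Debug.
; The construction script sizes the collider from the last definition and colored Miss, Great, Good and OK boxes from the first four.
; Deactivate disables the collider.
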(event OnComponentBeginOverlap(BoxCollider)
  (params (OverlappedComponent :type Primitive%20Component%20Object%20Reference) (OtherActor :type Actor%20Object%20Reference) (OtherComp :type Primitive%20Component%20Object%20Reference) (OtherBodyIndex :type Integer) (bFromSweep :type Boolean) (SweepResult :type Hit%20Result%20Structure%20%28by%20ref%29))
  (bind (_obstacleeventvalue _distance) (CallFunction|GetRegionValue (Transformation|GetActorLocation OtherActor)))
  (if (Variables|Default|GetDebug)
    (Development|PrintString (Utilities|String|Append (.RegionName (Utilities|Struct|BreakObstacleEventValue _obstacleeventvalue)) " " (Utilities|String|ToString(Float) _distance) " " (Utilities|String|ToString(Float) (.Distance (Utilities|Struct|BreakObstacleEventValue _obstacleeventvalue))) " " (Utilities|GetObjectName OtherActor)))))

(event Custom|Deactivate
  (Collision|SetCollisionEnabled (Variables|Default|GetBox%20Collider) "NoCollision"))

(fn ConstructionScript
  (bind _def (Variables|Default|GetDef))
  (bind _scoredefinitions (Variables|/Game/Obstacles/BP_ObstacleEventValueDefinition.BP_ObstacleEventValueDefinition_C|GetScoreDefinitions _def))
  (Components|Box|SetBoxExtent (Variables|Default|GetBox%20Collider) (Math|Vector|MakeVector 32.0 (.Distance (Utilities|Struct|BreakObstacleEventValue (Utilities|Array|Get(acopy) _scoredefinitions (- (Utilities|Array|Length _scoredefinitions) 1)))) 32.0) true)
  (CallFunction|SetDebugBox (Variables|Default|GetMiss) 0 4.0 (Math|Color|MakeColor 0 0 255 255))
  (CallFunction|SetDebugBox (Variables|Default|GetGreat) 1 3.0 (Math|Color|MakeColor 0 255 0 255))
  (CallFunction|SetDebugBox (Variables|Default|GetGood) 2 2.0 (Math|Color|MakeColor 0 255 255 255))
  (CallFunction|SetDebugBox (Variables|Default|GetOK) 3 1.0 (Math|Color|MakeColor 0 128 255 255)))

(fn SetDebugBox
  (params (Box :type Box%20Component%20Object%20Reference) (Index :type Integer) (LineThickness :type Float%20%28double-precision%29) (ShapeColor :type Color%20Structure))
  (Class|ShapeComponent|SetLineThickness Box LineThickness)
  (Variables|/Script/Engine.ShapeComponent|SetShapeColor Box ShapeColor)
  (Components|Box|SetBoxExtent Box (Math|Vector|MakeVector 32.0 (.Distance (Utilities|Struct|BreakObstacleEventValue (CallFunction|GetObstacleEventValue Index))) 32.0) true))

(fn GetObstacleEventValue
  (params (Index :type Integer))
  (return (Utilities|Array|Get(acopy) (Variables|/Game/Obstacles/BP_ObstacleEventValueDefinition.BP_ObstacleEventValueDefinition_C|GetScoreDefinitions (Variables|Default|GetDef)) Index)))

(fn GetRegionValue
  (params (Other%20Location :type Vector))
  (bind _returnvalue (Transformation|GetActorTransform))
  (bind _def (Variables|Default|GetDef))
  (bind _returnvalue_2 (Math|Transform|InverseTransformLocation _returnvalue Other%20Location))
  (bind _scoredefinitions (Variables|/Game/Obstacles/BP_ObstacleEventValueDefinition.BP_ObstacleEventValueDefinition_C|GetScoreDefinitions _def))
  (bind _y (Math|Vector|BreakVector _returnvalue_2))
  (bind _returnvalue_3 (Math|Float|Absolute(Float) _y))
  ;[0.15 0.15 0.15 0.5] 距離のリージョン判定
  (bind _array_element (Utilities|Array|ForEachLoopwithBreak _scoredefinitions)
    (:LoopBody
      (if (<= _returnvalue_3 (.Distance (Utilities|Struct|BreakObstacleEventValue _array_element)))
        (return _array_element _returnvalue_3)))
    (:Completed
      ;[0.15 0.15 0.15 0.5] とりあえずコライダーに接触したらスコア加算する
      (return (Utilities|Array|Get(acopy) _scoredefinitions (Utilities|Array|LastIndex _scoredefinitions)) _returnvalue_3))))